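; BP_PureCharacterVR is a VR player character that sets up floor-level tracking and spawns its two hands when play begins.
; On BeginPlay it spawns a left and a right BP_Hand as owned actors, assigns each its side, and attaches them to VRRoot.
; Tick, overlap and the construction script are empty, so this Blueprint handles setup only.
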(event EventBeginPlay
  (bind _returnvalue (Math|Transform|MakeTransform "0, 0, 0"))
  (bind _self self)
  (Class|HeadMountedDisplayFunctionLibrary|SetTrackingOrigin "Floor")
  (Utilities|FlowControl|Sequence
    (:then_0
      (bind _returnvalue_2 (Game|SpawnActorfromClass "/Game/BP_Hand.BP_Hand_C" _returnvalue "Undefined" _self 0))
      (Class|HandController|SetHand _returnvalue_2 "Left")
      (Transformation|AttachComponentToComponent _returnvalue_2 (Variables|Default|GetVRRoot) "None" "SnapToTarget" "SnapToTarget" "KeepWorld" false))
    (:then_1
      (bind _returnvalue_3 (Game|SpawnActorfromClass "/Game/BP_Hand.BP_Hand_C" _returnvalue "Undefined" _self 0))
      (Class|HandController|SetHand _returnvalue_3 "Right")
      (Transformation|AttachComponentToComponent _returnvalue_3 (Variables|Default|GetVRRoot) "None" "SnapToTarget" "SnapToTarget" "KeepWorld" false))))

(event Collision|EventActorBeginOverlap
  (params (OtherActor :type Actor%20Object%20Reference)))

(event EventTick
  (params (DeltaSeconds :type Float%20%28single-precision%29)))

(fn ConstructionScript)